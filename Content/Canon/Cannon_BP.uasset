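; Cannon actor that the player can fire while standing inside its trigger box.
; Overlap with a MixamoCharacter_Master enables input for player controller 0, and leaving disables it again.
; While input is enabled, pressing F spawns a CannonballProjectile_BP at the TargetPoint's transform, with no cooldown or ammo check.
; The construction script also calls DisableInput.
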(event OnComponentBeginOverlap(TriggerBox)
  (params (OtherActor :type Actor%20Object%20Reference) (OtherComp :type Primitive%20Component%20Object%20Reference) (OtherBodyIndex :type Integer) (bFromSweep :type Boolean) (SweepResult :type Hit%20Result%20Structure%20%28by%20ref%29))
  (Utilities|Casting|CastToMixamoCharacter_Master OtherActor)
  (Input|EnableInput (Game|GetPlayerController 0)))

(event OnComponentEndOverlap(TriggerBox)
  (params (OtherActor :type Actor%20Object%20Reference) (OtherComp :type Primitive%20Component%20Object%20Reference) (OtherBodyIndex :type Integer))
  (Utilities|Casting|CastToMixamoCharacter_Master OtherActor)
  (Input|DisableInput (Game|GetPlayerController 0)))

(event EventBeginPlay)

(event EventActorBeginOverlap
  (params (OtherActor :type Actor%20Object%20Reference)))

(event EventTick
  (params (DeltaSeconds :type Float%20%28single-precision%29)))

(event Input|KeyboardEvents|F
  (params (Key :type Key%20Structure :default "AnyKey"))
  (bind _targetpoint (Variables|Default|GetTargetPoint))
  (bind _returnvalue (Transformation|GetWorldTransform _targetpoint))
  (bind (_location _rotation _scale) (Math|Transform|BreakTransform _returnvalue))
  (:Pressed
    (Game|SpawnActorfromClass "/Game/Canon/Ball/CannonballProjectile_BP.CannonballProjectile_BP_C" (Math|Transform|MakeTransform _location _rotation (* _scale 1.0)) "Undefined" 0 0)))

(fn ConstructionScript
  (Input|DisableInput 0))