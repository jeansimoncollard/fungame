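; HillTree_02_BP is a choppable tree that falls and drops a log.
; CutTree checks that the owning Mixamo_Kachujin pawn's line trace hit this tree, then a timeline adds roll to it; BeginPlay runs a similar timeline.
; Both timelines start a do-once looping timer that randomly triggers destruction: capsule physics, a spawned Log and a delayed actor removal.
; Stop events clear the timer and halt the timelines.
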(event Custom|CutTree
  (bind _returnvalue (Transformation|GetActorRotation))
  (bind (_roll _pitch _yaw) (Math|Rotator|BreakRotator _returnvalue))
  (bind _aspawn (Utilities|Casting|CastToPawn (Components|GetOwner)))
  (bind _asmixamo_kachujin (Utilities|Casting|CastToMixamo_Kachujin _aspawn))
  (bind _ashill_tree_02_bp (Utilities|Casting|CastToHillTree_02_BP (.HitActor (Collision|BreakHitResult (Variables|/Game/MixamoAnimPack/Mixamo_Kachujin/Mixamo_Kachujin.Mixamo_Kachujin_C|GetHitLineTrace _asmixamo_kachujin)))))
  (if (and (== _ashill_tree_02_bp self) (.bBlockingHit (Collision|BreakHitResult (Variables|/Game/MixamoAnimPack/Mixamo_Kachujin/Mixamo_Kachujin.Mixamo_Kachujin_C|GetHitLineTrace _asmixamo_kachujin))))
    (bind _roll_2 (Timeline|Timeline_1 Play)
      (:Update
        (Transformation|SetActorRotation (Math|Rotator|MakeRotator (+ _roll _roll_2) _pitch _yaw))
        (CallFunction|TryDestroyTree)))))

(event Custom|StopCutTree_Copy_Copy
  (Utilities|FlowControl|DoOnce false) ; enters at Reset
)

(event Custom|StopCutTree
  (bind _returnvalue (Transformation|GetActorRotation))
  (bind (_roll _pitch _yaw) (Math|Rotator|BreakRotator _returnvalue))
  (CallFunction|StopCutTreeCopy)
  (Class|KismetSystemLibrary|ClearTimerHandle (Variables|Default|GetHandleToTimer))
  (bind _roll_2 (Timeline|Timeline_1 Stop)
    (:Update
      (Transformation|SetActorRotation (Math|Rotator|MakeRotator (+ _roll _roll_2) _pitch _yaw))
      (CallFunction|TryDestroyTree))))

(event Custom|TryDestroyTree
  (Utilities|FlowControl|DoOnce false
    (:Completed
      (bind _returnvalue (Utilities|Time|SetTimerbyFunctionName 0 "DestroyTree?" 1.5 true))
      (Variables|Default|SetHandleToTimer _returnvalue))))

(event Custom|StopCutTree_Copy
  (bind _returnvalue (Transformation|GetActorRotation))
  (bind (_roll _pitch _yaw) (Math|Rotator|BreakRotator _returnvalue))
  (CallFunction|StopCutTreeCopyCopy)
  (Class|KismetSystemLibrary|ClearTimerHandle (Variables|Default|GetHandleToTimer))
  (bind _roll_2 (Timeline|Timeline_0 Stop)
    (:Update
      (Transformation|SetActorRotation (Math|Rotator|MakeRotator (+ _roll _roll_2) _pitch _yaw))
      (bind _aspawn (Utilities|Casting|CastToPawn (Components|GetOwner)))
      (bind _asmixamo_character_master (Utilities|Casting|CastToMixamoCharacter_Master _aspawn))
      (bind _asmixamo_kachujin (Utilities|Casting|CastToMixamo_Kachujin _aspawn))
      (bind _returnvalue_2 (Utilities|Casting|CastToPlayerController (Pawn|GetController _asmixamo_character_master)))
      (Variables|Default|SetHitLineTrace (Variables|/Game/MixamoAnimPack/Mixamo_Kachujin/Mixamo_Kachujin.Mixamo_Kachujin_C|GetHitLineTrace _asmixamo_kachujin))
      (Input|EnableInput _returnvalue_2)
      (CallFunction|TryDestroyTree))))

(event Custom|Destroy%20tree
  (Physics|SetSimulatePhysics (Variables|Default|GetCapsulecollision) true)
  (Game|SpawnActorfromClass "/Game/Items/Actors/Log.Log_C" (Transformation|GetWorldTransform (Variables|Default|GetDropLocation)) "Undefined" 0 1 0)
  (Utilities|FlowControl|Delay (Math|Random|RandomFloatinRange 5.0 15.0))
  (Actor|DestroyActor))

(event EventBeginPlay
  (bind _returnvalue (Transformation|GetActorRotation))
  (bind (_roll _pitch _yaw) (Math|Rotator|BreakRotator _returnvalue))
  (bind _aspawn (Utilities|Casting|CastToPawn (Components|GetOwner)))
  (bind _roll_2 (Timeline|Timeline_0 Play)
    (:Update
      (Transformation|SetActorRotation (Math|Rotator|MakeRotator (+ _roll _roll_2) _pitch _yaw))
      (bind _aspawn_2 (Utilities|Casting|CastToPawn (Components|GetOwner)))
      (bind _asmixamo_character_master (Utilities|Casting|CastToMixamoCharacter_Master _aspawn_2))
      (bind _asmixamo_kachujin (Utilities|Casting|CastToMixamo_Kachujin _aspawn_2))
      (bind _returnvalue_2 (Utilities|Casting|CastToPlayerController (Pawn|GetController _asmixamo_character_master)))
      (Variables|Default|SetHitLineTrace (Variables|/Game/MixamoAnimPack/Mixamo_Kachujin/Mixamo_Kachujin.Mixamo_Kachujin_C|GetHitLineTrace _asmixamo_kachujin))
      (Input|EnableInput _returnvalue_2)
      (CallFunction|TryDestroyTree))))

(fn ConstructionScript)

(fn DestroyTree?
  (if (> (Math|Random|RandomIntegerinRange 0 10) 5)
    (CallFunction|DestroyTree)))